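; Player actor that moves on the X-Z plane from MoveX/MoveY axis input and opens with an animated spawn.
; On BeginPlay, a timeline raises it while spinning it in yaw, then sets MoveEnabled and caches BP_GameMode beforehand.
; The axis events ease horizontal and vertical speeds toward their targets through the shared Movement function.
; Tick applies each axis as a separate swept move and turns yaw against horizontal speed.
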(event EventBeginPlay
  ;[1 1 1] PlayerSpawnAnimation
  (bind _asbp_game_mode (Utilities|Casting|CastToBP_GameMode (Game|GetGameMode)))
  (Variables|Default|SetBP_GameMode _asbp_game_mode)
  (Variables|Default|SetYaw (.Yaw (Math|Rotator|BreakRotator (Transformation|GetActorRotation))))
  (Variables|Default|SetSpawnLocation (Transformation|GetActorLocation))
  (bind _speed (Timeline|SpawnAnimation Play)
    (:Update
      (Transformation|SetActorLocation (Math|Vector|Lerp(Vector) (Variables|Default|GetSpawnLocation) (+ (Variables|Default|GetSpawnLocation) "0, 0,60.000000") _speed) false false)
      (Transformation|SetActorRotation (Math|Rotator|Lerp(Rotator) "0, 0, 0" (Math|Rotator|MakeRotator 0.0 0.0 (+ (Variables|Default|GetYaw) 7.2e+02)) _speed)))
    (:Finished
      (Variables|Default|SetMoveEnabled true))))

(event EventTick
  (params (DeltaSeconds :type Float%20%28single-precision%29))
  ;[1 1 1] Movement
  (Variables|Default|SetDeltaSeconds DeltaSeconds)
  (Transformation|SetActorLocation (+ (Transformation|GetActorLocation) (Math|Vector|MakeVector (Variables|Default|GetHozSpeed) 0.0 0.0)) true false)
  (Transformation|SetActorLocation (+ (Transformation|GetActorLocation) (Math|Vector|MakeVector 0.0 0.0 (Variables|Default|GetVertSpeed))) true false)
  (Transformation|SetActorRotation (Class|KismetMathLibrary|RInterptoConstant (Transformation|GetActorRotation) (Math|Rotator|MakeRotator 0.0 0.0 (+ (* (Variables|Default|GetHozSpeed) -7.0) (Variables|Default|GetYaw))) (Variables|Default|GetDeltaSeconds) 8e+01)))

(event Input|AxisEvents|InputAxisMoveX
  (params (AxisValue :type Float%20%28single-precision%29))
  ;[1 1 1] PlayerInput
  (bind _returnvalue (CallFunction|Movement AxisValue (Variables|Default|GetHozSpeed)))
  (Variables|Default|SetHozSpeed _returnvalue))

(event Input|AxisEvents|InputAxisMoveY
  (params (AxisValue :type Float%20%28single-precision%29))
  ;[1 1 1] PlayerInput
  (bind _returnvalue (CallFunction|Movement AxisValue (Variables|Default|GetVertSpeed)))
  (Variables|Default|SetVertSpeed _returnvalue))

(fn ConstructionScript)

(fn Movement
  (params (Direction :type Float%20%28single-precision%29) (Speed :type Float%20%28single-precision%29))
  (return (Math|Interpolation|FInterpTo Speed (* (Variables|Default|GetMovementSpeed) Direction) (Variables|Default|GetDeltaSeconds) 6.0)))